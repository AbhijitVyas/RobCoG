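; BP_GreenBalls is an actor that sets its own scale and periodically prints the locations of static mesh actors in the level.
; The construction script scales it uniformly from the ScaleRND variable and makes an unused query for static mesh actors.
; BeginPlay waits on a short delay, enables collision, then prints each StaticMeshActor location.
; The loop body wires back into the delay, so the whole pass repeats indefinitely.
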(event EventBeginPlay
  (Utilities|FlowControl|Delay 1.0 :!label _label)
  (bind _outactors (Actor|GetAllActorsOfClass "/Script/Engine.StaticMeshActor"))
  (Collision|SetActorEnableCollision true)
  (for _array_element _outactors
    (Development|PrintString (Utilities|String|ToString(Vector) (Transformation|GetActorLocation _array_element)))
    (goto _label)))

(event Collision|EventActorBeginOverlap
  (params (OtherActor :type Actor%20Object%20Reference)))

(event EventTick
  (params (DeltaSeconds :type Float%20%28single-precision%29)))

(fn ConstructionScript
  (Actor|GetAllActorsOfClass "/Script/Engine.StaticMeshActor")
  (Transformation|SetActorRelativeScale3D (Math|Conversions|ToVector(Float) (* (Variables|Default|GetScaleRND) 5.0))))