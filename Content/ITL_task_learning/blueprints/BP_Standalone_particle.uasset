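; Standalone actor that receives exported particle data from its Niagara system and prints it on screen, apparently as a learning test.
; On BeginPlay it passes itself to Niagara through the User.BPCallBack object variable, so the system can call back into the Blueprint.
; The ParticleData event loops over the received particles, printing each index and position as text colored by that particle's velocity.
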(event EventBeginPlay
  (Niagara|SetNiagaraVariable(Object) (Variables|Default|GetNiagara) "User.BPCallBack" self))

(event Collision|EventActorBeginOverlap
  (params (OtherActor :type Actor%20Object%20Reference)))

(event EventTick
  (params (DeltaSeconds :type Float%20%28single-precision%29)))

(event EventParticleData
  (params (Data :type Array%20of%20Basic%20Particle%20Data%20Structures) (NiagaraSystem :type Niagara%20System%20Object%20Reference))
  (for (_array_element _array_index) Data
    (Development|PrintString (Utilities|String|Append (Utilities|String|ToString(Integer) _array_index) (Utilities|String|ToString(Vector) (.Position (Utilities|Struct|BreakBasicParticleData _array_element)))) true true (Math|Conversions|ToLinearColor(Vector) (.Velocity (Utilities|Struct|BreakBasicParticleData _array_element))) 1e+01)))

(fn ConstructionScript)